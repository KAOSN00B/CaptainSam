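; Parent display platform Blueprint that showcases a chosen Niagara effect inside a configurable room.
; The construction script assigns the effect, labels both text renders with its asset name, picks divider and wall meshes, and offsets the effect by particle type.
; Tick spins the pivot for trail effects and, when looping, calls Replay after a delay.
; Replay reactivates the system, optionally resetting it, only when ConstantUpdate is set.
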(event EventTick
  (params (DeltaSeconds :type Float%20%28single-precision%29))
  (Transformation|AddLocalRotation (Variables|Default|GetParticalPivot) (Math|Rotator|SelectRotator (Math|Rotator|MakeRotator 0.0 0.0 (* DeltaSeconds (Variables|Default|GetTrailRotationSpeed))) "0, 0, 0" (Variables|Default|GetIsTrail)) false false)
  ;[1 1 1] Timer
  (if (Variables|Default|GetLoopParticles)
    (Utilities|FlowControl|Delay (Variables|Default|GetReplayDelay))
    (CallFunction|Replay)))

(fn ConstructionScript
  (bind _startcap (Variables|Default|GetStartCap))
  (bind _endcap (Variables|Default|GetEndCap))
  (bind _sm_bld_divider_01 (Variables|Default|GetSM_Bld_Divider_01))
  (bind _sm_bld_divider_02 (Variables|Default|GetSM_Bld_Divider_02))
  (Class|NiagaraComponent|SetAsset (Variables|Default|GetNiagaraSystem) (Variables|Default|GetNiagara%20Effect) true)
  (Rendering|Components|TextRender|SetText (Variables|Default|GetTextRender) (Utilities|Text|ToText(String) (Utilities|GetObjectName (Effects|Components|ParticleSystem|GetFXSystemAsset (Variables|Default|GetNiagaraSystem)))))
  (CallFunction|Replay)
  (Rendering|SetVisibility _sm_bld_divider_01 (Utilities|Enum|NotEqual(Enum) _startcap "NewEnumerator0") false)
  (Components|StaticMesh|SetStaticMesh _sm_bld_divider_01 (Utilities|Select :Index _startcap :NewEnumerator0 0 :NewEnumerator1 "/Game/Assets/PolygonParticleFX/Meshes/Demo_Room/SM_Bld_Divider_01.SM_Bld_Divider_01" :NewEnumerator2 "/Game/Assets/PolygonParticleFX/Meshes/Demo_Room/SM_Bld_Divider_02.SM_Bld_Divider_02"))
  (Rendering|SetVisibility _sm_bld_divider_02 (Utilities|Enum|NotEqual(Enum) _endcap "NewEnumerator0") false)
  (Components|StaticMesh|SetStaticMesh _sm_bld_divider_02 (Utilities|Select :Index _endcap :NewEnumerator0 0 :NewEnumerator1 "/Game/Assets/PolygonParticleFX/Meshes/Demo_Room/SM_Bld_Divider_01.SM_Bld_Divider_01" :NewEnumerator2 "/Game/Assets/PolygonParticleFX/Meshes/Demo_Room/SM_Bld_Divider_02.SM_Bld_Divider_02"))
  (Components|StaticMesh|SetStaticMesh (Variables|Default|GetRoomMesh) (select (Variables|Default|GetCeilingHole) "/Game/Assets/PolygonParticleFX/Meshes/Demo_Room/SM_Bld_Wall_02.SM_Bld_Wall_02" "/Game/Assets/PolygonParticleFX/Meshes/Demo_Room/SM_Bld_Wall_01.SM_Bld_Wall_01"))
  (Transformation|SetRelativeLocation (Variables|Default|GetNiagaraSystem) (Utilities|Select :Index (Variables|Default|GetParticleType) :NewEnumerator0 (Math|Vector|MakeVector 0.0 0.0 (Variables|Default|GetNormalOffset)) :NewEnumerator1 (Math|Vector|MakeVector (Variables|Default|GetTrailRotationOffset) 0.0 (Variables|Default|GetTrailOffset)) :NewEnumerator2 (Math|Vector|MakeVector 0.0 0.0 (Variables|Default|GetAreaOffset))) false false))

(fn Replay
  (if (Variables|Default|GetConstantUpdate)
    (Components|Activation|SetActive (Variables|Default|GetNiagaraSystem) true (Variables|Default|GetResetOnReplay))))