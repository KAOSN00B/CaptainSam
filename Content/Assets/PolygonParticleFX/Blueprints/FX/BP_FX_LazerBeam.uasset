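; Laser beam effect Blueprint that fires a continuous line-traced beam from its Arrow component, starting at BeginPlay and updating every Tick.
; On a hit, it scales the beam mesh to the hit distance and shows the impact particle there.
; On a miss, it hides the impact and stretches a thinner beam to LaserLength.
; BeginPlay also clears RT_Damage and creates a Brush material instance, which this graph never uses.
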(event Custom|Fire_Lazer
  (bind _lazer_beam_hit (Variables|Default|GetLazer_Beam_Hit))
  (bind _arrow (Variables|Default|GetArrow))
  (bind _lazer_beam_hit_2 (Variables|Default|GetLazer_Beam_Hit))
  (bind _returnvalue (Transformation|GetWorldLocation _arrow))
  ;[1 1 1] LineTrace
  (bind (_outhit _returnvalue_2) (Collision|LineTraceByChannel _returnvalue (+ _returnvalue (* (Math|Vector|GetForwardVector _arrow) (Variables|Default|GetLaserLength))) "TraceTypeQuery1" true 0 "None"))
  (if _returnvalue_2
    ;[1 1 1] SpawnLaserMesh
    (Transformation|SetWorldScale3D (Variables|Default|GetLazer_Beam) (Math|Vector|MakeVector 1.0 1.0 (/ (Math|Vector|Distance(Vector) (.Location (Collision|BreakHitResult _outhit)) (.TraceStart (Collision|BreakHitResult _outhit))) 2e+01)))
    ;[1 1 1] SpawnHitParticle
    (Rendering|SetVisibility (Variables|Default|GetLazer_Beam) true false)
    (Components|Activation|SetActive (Variables|Default|GetFx_Lazer_Beam) true false)
    (Components|Activation|SetActive _lazer_beam_hit_2 true false)
    (Transformation|SetWorldLocation _lazer_beam_hit_2 (.Location (Collision|BreakHitResult _outhit)) false false)
    (Rendering|SetVisibility _lazer_beam_hit_2 true false)
    (else
      (Rendering|SetVisibility _lazer_beam_hit false false)
      (Components|Activation|SetActive _lazer_beam_hit false false)
      (Transformation|SetWorldScale3D (Variables|Default|GetLazer_Beam) (Math|Vector|MakeVector 0.1 0.1 (/ (Variables|Default|GetLaserLength) 2e+01))))))

(event EventBeginPlay
  ;[1 1 1] Create/Remove Brush
  (Rendering|ClearRenderTarget2D "/Game/Assets/PolygonParticleFX/Textures/RenderTargets/RT_Damage.RT_Damage")
  (bind _returnvalue (Rendering|Material|CreateDynamicMaterialInstance "/Game/Assets/PolygonParticleFX/Materials/MI_Particle_01.MI_Particle_01" "None" "None" :!class /Script/Engine.KismetMaterialLibrary))
  (Variables|Default|SetBrush _returnvalue)
  (CallFunction|FireLazer))

(event EventTick
  (params (DeltaSeconds :type Float%20%28single-precision%29))
  (CallFunction|FireLazer))

(fn ConstructionScript)